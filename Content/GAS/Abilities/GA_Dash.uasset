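; GA_Dash is a Gameplay Ability that makes the owning STUBaseCharacter dash and damages the actors it hits.
; On activation it calls TryDash on the character, which returns success and a list of damaged actors.
; On success it applies GE_DamageDash to each actor, then commits and ends; a failed cast or dash cancels the ability.
; Commit runs only after damage is applied, and debug prints report results.
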(event Ability|EventActivateAbility
  (bind _returnvalue (Ability|GetActorInfo))
  (bind _asstubase_character (Utilities|Casting|CastToSTUBaseCharacter (.owneractor _returnvalue))
    (:then
      (bind (_damagedactors _returnvalue_2) (Class|STUBaseCharacter|TryDash _asstubase_character))
      (Development|PrintString (Utilities|String|Append "Actors: " (Utilities|String|ToString(Integer) (Utilities|Array|Length _damagedactors)) " Dash " (Utilities|String|SelectString "Ok" "Bad" _returnvalue_2)))
      (if _returnvalue_2
        (for _array_element _damagedactors
          (GameplayEffects|ApplyGameplayEffectToTarget (Ability|GetAbilitySystemComponent (.owneractor _returnvalue)) "/Game/GAS/Effects/GE_DamageDash.GE_DamageDash_C" (Variables|/Script/My1stShootThemUp.STUBaseCharacter|GetAbilitySystemComponent _array_element) 1.0 (Utilities|Struct|MakeGameplayEffectContextHandle))
          (Development|PrintString (Utilities|String|ToString(Float) (.ReturnValue (Ability|Attribute|GetFloatAttributefromAbilitySystemComponent (Variables|/Script/My1stShootThemUp.STUBaseCharacter|GetAbilitySystemComponent _array_element) "(AttributeName=\"IsStunt\",Attribute=/Script/My1stShootThemUp.CharacterAttributeSet:IsStunt,AttributeOwner=None)")))))
        (Ability|CommitAbility)
        (Ability|EndAbility)
        (else
          (Ability|CancelAbility))))
    (:CastFailed
      (Ability|CancelAbility))))

(event Ability|EventOnEndAbility
  (params (bWasCancelled :type Boolean)))