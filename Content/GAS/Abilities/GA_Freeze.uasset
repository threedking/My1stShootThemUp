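; GA_Freeze is a Gameplay Ability that lets the owning STUBaseCharacter perform a frost attack on other actors.
; It plays the AM_Frost montage, gets the affected actors from the character's Freeze function, and applies the GE_Frost effect to each through the ability system.
; It prints debug counts and attribute values, then commits only after applying effects and ends, or cancels if the owner cast fails.
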(event Ability|EventActivateAbility
  (bind _returnvalue (Ability|GetActorInfo))
  (bind _asstubase_character (Utilities|Casting|CastToSTUBaseCharacter (.owneractor _returnvalue))
    (:then
      (Animation|PlayAnimMontage _asstubase_character "/Game/Player/Animations/AM_Frost.AM_Frost" 1.0 "None")
      (bind _returnvalue_2 (Class|STUBaseCharacter|Freeze _asstubase_character))
      (Development|PrintString (Utilities|String|Append "Frozen Actors: " (Utilities|String|ToString(Integer) (Utilities|Array|Length _returnvalue_2))))
      (for _array_element _returnvalue_2
        (GameplayEffects|ApplyGameplayEffectToTarget (Ability|GetAbilitySystemComponent (.owneractor _returnvalue)) "/Game/GAS/Effects/GE_Frost.GE_Frost_C" (Variables|/Script/My1stShootThemUp.STUBaseCharacter|GetAbilitySystemComponent _array_element) 1.0 (Utilities|Struct|MakeGameplayEffectContextHandle))
        (if (.bSuccessfullyFoundAttribute (Ability|Attribute|GetFloatAttributefromAbilitySystemComponent (Variables|/Script/My1stShootThemUp.STUBaseCharacter|GetAbilitySystemComponent _array_element) "(AttributeName=\"Frost\",Attribute=/Script/My1stShootThemUp.CharacterAttributeSet:Frost,AttributeOwner=None)"))
          (Development|PrintString (Utilities|String|Append "Frost: " (Utilities|String|ToString(Float) (.ReturnValue (Ability|Attribute|GetFloatAttributefromAbilitySystemComponent (Variables|/Script/My1stShootThemUp.STUBaseCharacter|GetAbilitySystemComponent _array_element) "(AttributeName=\"Frost\",Attribute=/Script/My1stShootThemUp.CharacterAttributeSet:Frost,AttributeOwner=None)")))))))
      (Ability|CommitAbility)
      (Ability|EndAbility))
    (:CastFailed
      (Ability|CancelAbility))))

(event Ability|EventOnEndAbility
  (params (bWasCancelled :type Boolean)))