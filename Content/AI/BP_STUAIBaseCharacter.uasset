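; BP_STUAIBaseCharacter is a base AI character Blueprint that shows health, frost and stun changes visually.
; Health changes update the WBP_AIHealthBar in its HealthWidget as a fraction of 100 and hide the bar at zero.
; Stun changes are forwarded to the same widget.
; Frost changes drive the "Frost" scalar parameter through a dynamic material instance created on the mesh's first material slot at each event.
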(event Collision|EventActorBeginOverlap
  (params (OtherActor :type Actor%20Object%20Reference)))

(event EventTick
  (params (DeltaSeconds :type Float%20%28single-precision%29)))

(event EventOnHealthChangedBP
  (params (Health :type Float%20%28single-precision%29))
  (bind _returnvalue (/ Health 1e+02))
  (bind _aswbp_aihealth_bar (Utilities|Casting|CastToWBP_AIHealthBar (UserInterface|GetUserWidgetObject (Variables|Default|GetHealthWidget))))
  (Default|SetHealth _aswbp_aihealth_bar _returnvalue)
  (if true
    (Widget|SetVisibility _aswbp_aihealth_bar (select (> _returnvalue 0.0) "Visible" "Hidden"))))

(event EventOnStuntChangedBP
  (params (IsStunt :type Boolean))
  (bind _aswbp_aihealth_bar (Utilities|Casting|CastToWBP_AIHealthBar (UserInterface|GetUserWidgetObject (Variables|Default|GetHealthWidget))))
  (Default|ChangeStunt _aswbp_aihealth_bar IsStunt))

(event EventOnFrostChangedBP
  (params (Frost :type Float%20%28single-precision%29))
  (bind _mesh (Variables|Character|GetMesh))
  (bind _returnvalue (Rendering|Material|CreateDynamicMaterialInstance _mesh 0 (Rendering|Material|GetMaterial _mesh 0) "None" :!class /Script/Engine.PrimitiveComponent))
  (Rendering|Material|SetScalarParameterValue _returnvalue "Frost" Frost :!class /Script/Engine.MaterialInstanceDynamic))

(fn ConstructionScript)