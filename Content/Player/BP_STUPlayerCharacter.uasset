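; Player character Blueprint that adds an aim camera transition while the right mouse button is held.
; AimTimeline drives the spring arm's target length and camera lag speed, playing forward on press and reversing on release.
; The timeline runs at double rate into aim and normal rate back out, and an interrupted transition continues from its current position.
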(event Input|MouseEvents|RightMouseButton
  (params (Key :type Key%20Structure :default "None"))
  (bind _aim_timeline (Variables|Default|GetAim%20Timeline))
  (:Pressed
    (Components|Timeline|SetPlayRate _aim_timeline 2.0)
    (bind (_direction _arm_length _arm_speed) (Timeline|Aim%20Timeline Play)
      (:Update
        (Variables|/Script/Engine.SpringArmComponent|SetTargetArmLength (Variables|Default|GetSpringArmComponent) _arm_length)
        (Variables|/Script/Engine.SpringArmComponent|SetCameraLagSpeed (Variables|Default|GetSpringArmComponent) _arm_speed))))
  (:Released
    (Components|Timeline|SetPlayRate _aim_timeline 1.0)
    (Timeline|Aim%20Timeline Reverse)))

(fn ConstructionScript)